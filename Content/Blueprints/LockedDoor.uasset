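; LockedDoor is a coin-gated door for a side-scroller that opens once enough coins are collected.
; Its construction script builds the coins-needed label and stores the starting positions of three mesh pieces.
; A sphere overlap compares the SideScrollerGameMode coin count to the requirement, hiding the label when met.
; The DoorOpen timeline then moves each piece along Z using its own track, scaled by a shared distance.
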(event OnComponentBeginOverlap(Sphere)
  (params (OverlappedComponent :type Primitive%20Component%20Object%20Reference) (OtherActor :type Actor%20Object%20Reference) (OtherComp :type Primitive%20Component%20Object%20Reference) (OtherBodyIndex :type Integer) (bFromSweep :type Boolean) (SweepResult :type Hit%20Result%20Structure%20%28by%20ref%29))
  (bind _piecemovedistance (Variables|Default|GetpieceMoveDistance))
  (bind _asside_scroller_game_mode (Utilities|Casting|CastToSideScrollerGameMode (Game|GetGameMode))
    (:then
      (if (>= (Variables|/Game/Blueprints/SideScrollerGameMode.SideScrollerGameMode_C|Getcoins _asside_scroller_game_mode) (Variables|Default|GetCoinsNeededToOpen))
        (Rendering|SetVisibility (Variables|Default|GetTextRender) false false)
        (bind (_direction _piece_1 _piece_2 _piece_3) (Timeline|Door%20Open Play)
          (:Update
            (Transformation|SetRelativeLocation (Variables|Default|GetStaticMesh2) (+ (Variables|Default|GetstartingPosition2) (Math|Vector|MakeVector 0.0 0.0 (* _piece_2 _piecemovedistance))) false false)
            (Transformation|SetRelativeLocation (Variables|Default|GetStaticMesh1) (+ (Variables|Default|GetstartingPosition1) (Math|Vector|MakeVector 0.0 0.0 (* _piece_1 _piecemovedistance))) false false)
            (Transformation|SetRelativeLocation (Variables|Default|GetStaticMesh3) (+ (Variables|Default|GetstartingPosition3) (Math|Vector|MakeVector 0.0 0.0 (* _piece_3 _piecemovedistance))) false false)))))
    (:CastFailed
      (Development|PrintString "Wrong Game Mode"))))

(fn ConstructionScript
  (Rendering|Components|TextRender|SetText (Variables|Default|GetTextRender) (Utilities|Text|ToText(String) (Utilities|String|Append (Utilities|String|ToString(Integer) (Variables|Default|GetCoinsNeededToOpen)) " Coins 
Needed")))
  (Variables|Default|SetstartingPosition1 (Variables|/Script/Engine.SceneComponent|GetRelativeLocation (Variables|Default|GetStaticMesh1)))
  (Variables|Default|SetstartingPosition2 (Variables|/Script/Engine.SceneComponent|GetRelativeLocation (Variables|Default|GetStaticMesh2)))
  (Variables|Default|SetstartingPosition3 (Variables|/Script/Engine.SceneComponent|GetRelativeLocation (Variables|Default|GetStaticMesh3))))