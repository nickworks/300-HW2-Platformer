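; Mover actor that moves a static mesh along a spline, stopping at the end or, in Ping Pong mode, reversing after a pause at each end.
; On BeginPlay, Initialize converts OffsetPercent into a phase within the round trip, setting start time, delay and direction.
; While IsPlaying, Tick advances or rewinds time by state, then remaps normalized time through SpeedCurve to place the mesh on the spline.
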(event Custom|QueueForward
  (params (firstTime :type Boolean))
  (Utilities|FlowControl|Delay (select firstTime 0.0 (Variables|Default|GettimeDelayAtBothEnds)))
  (Variables|Default|SetcurrentState "NewEnumerator0"))

(event Custom|QueueReverse
  (Utilities|FlowControl|Delay (Variables|Default|GettimeDelayAtBothEnds))
  (Variables|Default|SetcurrentState "NewEnumerator1"))

(event EventBeginPlay
  (bind (_delaybeforeplaying _statetoswitchto) (CallFunction|Initialize))
  (Utilities|FlowControl|Delay _delaybeforeplaying)
  (Variables|Default|SetcurrentState _statetoswitchto))

(event EventTick
  (params (DeltaSeconds :type Float%20%28single-precision%29))
  (if (Variables|Default|GetisPlaying)
    (CallFunction|UpdateTime)
    (CallFunction|CalculateMeshPosition)))

(fn ConstructionScript)

(fn UpdateTime
  (bind _returnvalue (Utilities|Time|GetWorldDeltaSeconds))
  (bind _timetocomplete (Variables|Default|GettimeToComplete))
  (switch Utilities|FlowControl|Switch|SwitchonMoverState (Variables|Default|GetcurrentState)
    (:NewEnumerator0
      (bind _output_get (Variables|Default|SetcurrentTime (+ (Variables|Default|GetcurrentTime) _returnvalue)))
      (if (> _output_get _timetocomplete)
        (Variables|Default|SetcurrentState "NewEnumerator3")
        (Variables|Default|SetcurrentTime _timetocomplete)
        (switch Utilities|FlowControl|Switch|SwitchonMoverType (Variables|Default|GetmoverType)
          (:NewEnumerator1
            (CallFunction|QueueReverse)))))
    (:NewEnumerator1
      (bind _output_get_2 (Variables|Default|SetcurrentTime (- (Variables|Default|GetcurrentTime) _returnvalue)))
      (if (< _output_get_2 0.0)
        (Variables|Default|SetcurrentState "NewEnumerator2")
        (Variables|Default|SetcurrentTime 0.0)
        (switch Utilities|FlowControl|Switch|SwitchonMoverType (Variables|Default|GetmoverType)
          (:NewEnumerator1
            (CallFunction|QueueForward false)))))))

(fn CalculateMeshPosition
  (Transformation|SetRelativeLocation (Variables|Default|GetStaticMesh) (Spline|GetLocationatTime (Variables|Default|GetSpline) (Math|Curves|GetFloatValue (Variables|Default|GetSpeedCurve) (Math|Float|Clamp(Float) (/ (Variables|Default|GetcurrentTime) (Variables|Default|GettimeToComplete)))) "Local" false) false false))

(fn Initialize
  (bind _timedelayatbothends (Variables|Default|GettimeDelayAtBothEnds))
  (bind _timetocomplete (Variables|Default|GettimeToComplete))
  (bind _timetocomplete_2 (Variables|Default|GettimeToComplete))
  (bind _returnvalue (+ _timetocomplete_2 _timedelayatbothends))
  (LocalVariables|SetSecondsDelay (* (Variables|Default|GetoffsetPercent) _returnvalue 2.0))
  (if (< (Variables|Default|GetoffsetPercent) 0.5)
    (if (< (LocalVariables|GetSecondsDelay) (Variables|Default|GettimeDelayAtBothEnds))
      (return (- (Variables|Default|GettimeDelayAtBothEnds) (LocalVariables|GetSecondsDelay)) "NewEnumerator0")
      (else
        (Variables|Default|SetcurrentTime (- (LocalVariables|GetSecondsDelay) (Variables|Default|GettimeDelayAtBothEnds)))
        (return 0.0 "NewEnumerator0")))
    (else
      (LocalVariables|SetSecondsDelay (- (LocalVariables|GetSecondsDelay) _returnvalue))
      (if (< (LocalVariables|GetSecondsDelay) (Variables|Default|GettimeDelayAtBothEnds))
        (Variables|Default|SetcurrentTime _timetocomplete)
        (return (- (Variables|Default|GettimeDelayAtBothEnds) (LocalVariables|GetSecondsDelay)) "NewEnumerator1")
        (else
          (Variables|Default|SetcurrentTime (- _timetocomplete (- (LocalVariables|GetSecondsDelay) (Variables|Default|GettimeDelayAtBothEnds))))
          (return 0.0 "NewEnumerator1"))))))