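; One-way platform in wood and cloud variants that the player can pass through and drop off by crouching.
; The mesh ignores Pawns until the player enters the trigger box above it uncrouched, with a short delay when arriving from below.
; Crouch input or leaving the box turns collision off again.
; The construction script sets mesh and material by type, temporarily zeroing rotation to fit the trigger to the mesh bounds.
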(event OnComponentBeginOverlap(Box)
  (params (OverlappedComponent :type Primitive%20Component%20Object%20Reference) (OtherActor :type Actor%20Object%20Reference) (OtherComp :type Primitive%20Component%20Object%20Reference) (OtherBodyIndex :type Integer) (bFromSweep :type Boolean) (SweepResult :type Hit%20Result%20Structure%20%28by%20ref%29))
  (bind _returnvalue (Game|GetPlayerCharacter 0))
  (if (== OtherActor _returnvalue)
    (if (> (.z (Transformation|GetWorldLocation (Variables|/Script/Engine.Character|GetMesh _returnvalue))) (.z (Transformation|GetWorldLocation (Variables|Default|GetMesh))))
      _
      (else
        (Utilities|FlowControl|Delay 0.2)))
    (CallFunction|CollisionON)))

(event OnComponentEndOverlap(Box)
  (params (OverlappedComponent :type Primitive%20Component%20Object%20Reference) (OtherActor :type Actor%20Object%20Reference) (OtherComp :type Primitive%20Component%20Object%20Reference) (OtherBodyIndex :type Integer))
  (if (== OtherActor (Game|GetPlayerCharacter 0))
    (Utilities|FlowControl|Sequence
      (:then_0
        _)
      (:then_1
        (Utilities|FlowControl|Delay 0.2)
        (Input|DisableInput (Game|GetPlayerController 0))))
    (CallFunction|CollisionOFF)))

(event EventBeginPlay
  (CallFunction|CollisionOFF))

(event Input|ActionEvents|InputActionCrouch
  (params (Key :type Key%20Structure))
  (:Pressed
    (CallFunction|CollisionOFF)))

(fn ConstructionScript
  (bind _one_way_type (Variables|Default|GetOne%20Way%20Type))
  (bind _mesh (Variables|Default|GetMesh))
  (Utilities|FlowControl|Sequence
    (:then_0
      ;[1 1 1] Swap out the mesh
      (Components|StaticMesh|SetStaticMesh _mesh (Utilities|Select :Index _one_way_type :NewEnumerator0 "/Game/ArtKit/Platformer/Meshes/Fencing_Scaffolding/Pl_Woodcatwalk_4m_02.Pl_Woodcatwalk_4m_02" :NewEnumerator1 "/Game/ArtKit/Platformer/Meshes/Fencing_Scaffolding/Pl_Woodcatwalk_4m_01.Pl_Woodcatwalk_4m_01" :NewEnumerator4 "/Game/ArtKit/Platformer/Meshes/Fencing_Scaffolding/Pl_woodPlat_2m.Pl_woodPlat_2m" :NewEnumerator2 "/Game/ArtKit/Platformer/Meshes/Pl_CloudPlat_4x8m.Pl_CloudPlat_4x8m" :NewEnumerator3 "/Game/ArtKit/Platformer/Meshes/Pl_CloudPlat_8m.Pl_CloudPlat_8m"))
      (Rendering|Material|SetMaterial _mesh 0 (Utilities|Select :Index _one_way_type :NewEnumerator0 "/Game/ArtKit/Platformer/Materials/M_Wood_Yellow_Instance.M_Wood_Yellow_Instance" :NewEnumerator1 "/Game/ArtKit/Platformer/Materials/M_Wood_Yellow_Instance.M_Wood_Yellow_Instance" :NewEnumerator4 "/Game/ArtKit/Platformer/Materials/M_Wood_Yellow_Instance.M_Wood_Yellow_Instance" :NewEnumerator2 "/Game/ArtKit/Platformer/Materials/M_Cloud.M_Cloud" :NewEnumerator3 "/Game/ArtKit/Platformer/Materials/M_Cloud.M_Cloud")))
    (:then_1
      (LocalVariables|SetCachedRotation (Transformation|GetActorRotation))
      (Transformation|SetActorRotation "0, 0, 0" true))
    (:then_2
      (CallFunction|PositiontheTrigger))
    (:then_3
      (Transformation|SetActorRotation (LocalVariables|GetCachedRotation) true))))

(fn PositiontheTrigger
  (bind _edge_margin_size (Variables|Default|GetEdge%20Margin%20Size))
  (bind _mesh (Variables|Default|GetMesh))
  (bind (_origin _boxextent) (Collision|GetComponentBounds _mesh))
  (bind (_x _y _z) (Math|Vector|BreakVector _boxextent))
  (bind (_x_2 _y_2 _z_2) (Math|Vector|BreakVector _origin))
  (Utilities|FlowControl|Sequence
    (:then_0
      (Transformation|SetWorldLocation (Variables|Default|GetBox) (Math|Vector|MakeVector _x_2 _y_2 (+ _z_2 (Variables|Default|GetTrigger%20Offset) _z (Variables|Default|GetTrigger%20Thickness))) false true))
    (:then_1
      (Components|Box|SetBoxExtent (Variables|Default|GetBox) (Math|Vector|MakeVector (- _x _edge_margin_size) (- _y _edge_margin_size) (Variables|Default|GetTrigger%20Thickness)) true))))

(fn CollisionOFF
  (Collision|SetCollisionResponsetoChannel (Variables|Default|GetMesh) "ECC_Pawn" "ECR_Ignore")
  (Input|DisableInput (Game|GetPlayerController 0) 0))

(fn CollisionON
  (if (not (AI|Components|NavMovement|IsCrouching (Variables|/Script/Engine.Character|GetCharacterMovement (Game|GetPlayerCharacter 0))))
    (Collision|SetCollisionResponsetoChannel (Variables|Default|GetMesh) "ECC_Pawn" "ECR_Block")
    (Input|EnableInput (Game|GetPlayerController 0))))